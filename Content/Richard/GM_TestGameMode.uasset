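; Game mode for a record-and-replay button puzzle: the player records several characters in turn, then they act together.
; During tracking, a button press moves the player pawn to the next character's start and resets the tick counter, or starts replay after the last.
; Replay spawns three possessed replay characters, feeds them tick-indexed inputs from BPActionTracker, and signals completion when a press leaves all color buttons triggered.
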(event `self.ReceiveBeginPlay`
  (`GameplayStatics.CreatePlayer` 0)
  (bind _returnvalue (`|SpawnActorFromClass` "/Game/Richard/BP_TestCharacter.BP_TestCharacter_C" (`self.GetTransform` (`self.K2_FindPlayerStart` null "0")) "Undefined" "MultiplyWithRoot" null null))
  (bind _output_get (set `self.player_char` _returnvalue))
  (`Controller.Possess` (`GameplayStatics.GetPlayerController` 0) _output_get)
  (`KismetSystemLibrary.DelayUntilNextTick`)
  (`self.start_tracking`))

(event `self.ReceiveTick`
  (params (DeltaSeconds :type "Float (single-precision)"))
  (switch `/Game/Richard/E_InputTrackingStates` (`self.state`)
    (:`NewEnumerator0`
      (`self.advance_tick`))
    (:`NewEnumerator2`
      (`self.on_replay`)
      (`self.advance_tick`))))

(event `all_buttons_pressed_Event`
  (set `self.all_goals_complete` true))

(fn `advance_tick`
  (set `self.tick_n` (+ (`self.tick_n`) 1)))

(fn `is_time_reached`
  (returns (time_reached :type Boolean))
  (return (>= (`self.tick_n`) (`self.tick_to_end_on`))))

(fn `on_button_pressed`
  (params (character_id :type Integer))
  (locals (all_pressed :type Boolean))
  (set `local.all_pressed` false)
  (switch `/Game/Richard/E_InputTrackingStates` (`self.state`)
    (:`NewEnumerator0`
      (if (== (`local.character_id`) (- (`self.n_characters`) 1))
        (`self.start_replay`)
        (else
          (`self.switch_characters` (+ (`local.character_id`) 1)))))
    (:`NewEnumerator2`
      (bind _outactors (`GameplayStatics.GetAllActorsOfClass` "/Game/Richard/BP_ColorButton.BP_ColorButton_C"))
      (for _array_element _outactors
        (if (`/Game/Richard/BP_ColorButton.is_triggered` _array_element)
          (set `local.all_pressed` true)
          (else
            (set `local.all_pressed` false)
            (break))))
      (if (`local.all_pressed`)
        (`KismetSystemLibrary.PrintString` "All buttons pressed!!!")
        (`self.all_buttons_pressed`)))))

(fn `on_replay`
  (bind _outactors (`GameplayStatics.GetAllActorsOfClass` "/Game/Richard/BP_ReplayCharacter.BP_ReplayCharacter_C"))
  (for _array_element _outactors
    (bind _input (`/Game/Richard/Blueprints/BP_ActionTracker.get_input` (`self.BP_ActionTracker`) (`self.tick_n`) (`/Game/Richard/BP_ReplayCharacter.character_id` _array_element)))
    (`/Game/Richard/BP_ReplayCharacter.execute_input` _array_element _input))
  (bind _all_inputs_used (`/Game/Richard/Blueprints/BP_ActionTracker.are_all_inputs_used` (`self.BP_ActionTracker`) (`self.tick_n`)))
  (if _all_inputs_used
    (`KismetSystemLibrary.PrintString` "All inputs are used!!")))

(fn `spawn_replay_character`
  (params (character_id :type Integer))
  (returns (NewParam :type "/Game/Richard/BP_ReplayCharacter Object Reference"))
  (bind _returnvalue (+ character_id 1))
  (`GameplayStatics.CreatePlayer` _returnvalue)
  (bind _returnvalue_2 (`|SpawnActorFromClass` "/Game/Richard/BP_ReplayCharacter.BP_ReplayCharacter_C" (`self.GetTransform` (`self.K2_FindPlayerStart` null (`KismetStringLibrary.Conv_IntToString` character_id))) "Undefined" "MultiplyWithRoot" null null))
  (`Controller.Possess` (`GameplayStatics.GetPlayerController` _returnvalue) _returnvalue_2)
  (set `/Game/Richard/BP_ReplayCharacter.character_id` (`local.character_id`) _returnvalue_2)
  (return _returnvalue_2))

(fn `start_replay`
  (bind _outactors (`GameplayStatics.GetAllActorsOfClass` "/Game/Richard/BP_ColorButton.BP_ColorButton_C"))
  (for _array_element _outactors
    (set `/Game/Richard/BP_ColorButton.is_triggered` false _array_element))
  (`/Game/Richard/BP_TestCharacter.set_idle` (`self.player_char`))
  (set `self.tick_n` 0)
  (set `self.state` "NewEnumerator2")
  (for _index (range 3)
    (`self.spawn_replay_character` _index))
  (bind _outactors_2 (`GameplayStatics.GetAllActorsOfClass` "/Game/Richard/BP_TestCharacter.BP_TestCharacter_C"))
  (for _array_element_2 _outactors_2
    (`self.K2_DestroyActor` _array_element_2)))

(fn `start_tracking`
  (`/Game/Richard/Blueprints/BP_ActionTracker.reset` (`self.BP_ActionTracker`))
  (set `self.state` "NewEnumerator0")
  (set `self.tick_n` 0)
  (bind _outactors (`GameplayStatics.GetAllActorsOfClass` "/Game/Richard/BP_ReplayCharacter.BP_ReplayCharacter_C"))
  (for _array_element _outactors
    (`self.K2_DestroyActor` _array_element))
  (`/Game/Richard/BP_TestCharacter.set_tracking` (`self.player_char`) 0)
  (set `self.all_goals_complete` false))

(fn `switch_characters`
  (params (current_character :type Integer))
  (bind _player_char (`self.player_char`))
  (`self.K2_SetActorTransform` (`self.player_char`) (`self.GetTransform` (`self.K2_FindPlayerStart` null (`KismetStringLibrary.Conv_IntToString` current_character))) false false)
  (`/Game/Richard/BP_TestCharacter.set_character_id` _player_char (`/Game/Richard/BP_TestCharacter.character_id` _player_char))
  (`/Game/Richard/BP_TestCharacter.set_tracking` (`self.player_char`) current_character)
  (set `self.tick_n` 0))

(fn `UserConstructionScript`)
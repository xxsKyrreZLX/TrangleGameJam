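; Color-coded pressure button that only responds to the character whose CharacterId matches its own, showing red, green or blue for IDs 0 to 2.
; A matching test character entering the Box sets IsTriggered and notifies the test game mode; leaving clears the flag after a short delay.
; A separate ReplayOverlap volume lets a matching replay character set and immediately clear the flag without notifying the game mode.
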(event `self.ReceiveBeginPlay`
  (bind _character_id (`self.character_id`))
  (bind _asgm_test_game_mode (cast `/Game/Richard/GM_TestGameMode` (`GameplayStatics.GetGameMode`)))
  (set `self.game_mode` _asgm_test_game_mode)
  (if (== _character_id 0)
    (`PrimitiveComponent.SetMaterial` (`self.Cylinder`) 0 "/Game/Nawwaf/Materials/MI_ButtonRed.MI_ButtonRed")
    (elif (== _character_id 1)
      (`PrimitiveComponent.SetMaterial` (`self.Cylinder`) 0 "/Game/Nawwaf/Materials/MI_ButtonGreen.MI_ButtonGreen")
      (elif (== _character_id 2)
        (`PrimitiveComponent.SetMaterial` (`self.Cylinder`) 0 "/Game/Nawwaf/Materials/MI_ButtonBlue.MI_ButtonBlue")))))

(event `self.ReplayOverlap.OnComponentBeginOverlap`
  (params (OverlappedComponent :type "PrimitiveComponent Object Reference") (OtherActor :type "Actor Object Reference") (OtherComp :type "PrimitiveComponent Object Reference") (OtherBodyIndex :type Integer) (bFromSweep :type Boolean) (SweepResult :type "HitResult Structure (by ref)"))
  (bind _asbp_replay_character (cast `/Game/Richard/BP_ReplayCharacter` OtherActor))
  (if (== (`self.character_id`) (`/Game/Richard/BP_ReplayCharacter.character_id` _asbp_replay_character))
    (set `self.is_triggered` true)))

(event `self.Box.OnComponentBeginOverlap`
  (params (OverlappedComponent :type "PrimitiveComponent Object Reference") (OtherActor :type "Actor Object Reference") (OtherComp :type "PrimitiveComponent Object Reference") (OtherBodyIndex :type Integer) (bFromSweep :type Boolean) (SweepResult :type "HitResult Structure (by ref)"))
  (bind _asbp_test_character (cast `/Game/Richard/BP_TestCharacter` OtherActor))
  (if (== (`/Game/Richard/BP_TestCharacter.character_id` _asbp_test_character) (`self.character_id`))
    (`self.on_triggered`)))

(event `self.Box.OnComponentEndOverlap`
  (params (OverlappedComponent :type "PrimitiveComponent Object Reference") (OtherActor :type "Actor Object Reference") (OtherComp :type "PrimitiveComponent Object Reference") (OtherBodyIndex :type Integer))
  (bind _asbp_test_character (cast `/Game/Richard/BP_TestCharacter` OtherActor))
  (if (== (`/Game/Richard/BP_TestCharacter.character_id` _asbp_test_character) (`self.character_id`))
    (`KismetSystemLibrary.Delay` 0.5)
    (`self.on_character_exited`)))

(event `self.ReplayOverlap.OnComponentEndOverlap`
  (params (OverlappedComponent :type "PrimitiveComponent Object Reference") (OtherActor :type "Actor Object Reference") (OtherComp :type "PrimitiveComponent Object Reference") (OtherBodyIndex :type Integer))
  (bind _asbp_replay_character (cast `/Game/Richard/BP_ReplayCharacter` OtherActor))
  (if (== (`self.character_id`) (`/Game/Richard/BP_ReplayCharacter.character_id` _asbp_replay_character))
    (set `self.is_triggered` false)))

(fn `change_color`
  (params (Color :type Name) (MI :type "MaterialInstance Object Reference"))
  (if (`self.ActorHasTag` Color)
    (`PrimitiveComponent.SetMaterial` (`self.Cylinder`) 0 MI)))

(fn `on_character_exited`
  (set `self.is_triggered` false))

(fn `on_triggered`
  (set `self.is_triggered` true)
  (`/Game/Richard/GM_TestGameMode.on_button_pressed` (`self.game_mode`) (`self.character_id`)))

(fn `UserConstructionScript`)
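; BP_InputTracker records inputs into a single flat array and serves them back by tick and character index.
; TrackInput appends an entry to TrackedInputs, and Reset clears the array.
; GetInput treats the array as three equal, consecutive per-character blocks, offsetting the tick by the character index times one third of the array length.
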(fn `get_input`
  (params (tick :type Integer) (character :type Integer))
  (returns (NewParam :type "/Game/Richard/S_InputStruct Structure"))
  (return (`|GetArrayItem` (`self.tracked_inputs`) (+ tick (* character (/ (`KismetArrayLibrary.Array_Length` (`self.tracked_inputs`)) 3))))))

(fn `reset`
  (`KismetArrayLibrary.Array_Clear` (`self.tracked_inputs`)))

(fn `track_input`
  (params (inputs :type "/Game/Richard/S_InputStruct Structure"))
  (`KismetArrayLibrary.Array_Add` (`self.tracked_inputs`) inputs))
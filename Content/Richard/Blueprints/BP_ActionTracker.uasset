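; BP_ActionTracker records per-tick inputs for up to three characters, which can be read back by tick index.
; TrackInput appends each input to that character's own array, and Reset clears all three.
; GetInput returns the stored input for a character and tick, or an empty input once that array runs out.
; AreAllInputsUsed reports when a tick is past the end of every recording.
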(fn `_get_input_for`
  (params (input_array :type "Array of /Game/Richard/S_InputStruct Structure") (tick :type Integer))
  (returns (input :type "/Game/Richard/S_InputStruct Structure"))
  (locals (empty_input :type "/Game/Richard/S_InputStruct Structure"))
  (if (>= tick (`KismetArrayLibrary.Array_Length` input_array))
    (return (`local.empty_input`))
    (else
      (return (`|GetArrayItem` input_array tick)))))

(fn `are_all_inputs_used`
  (params (tick :type Integer))
  (returns (all_inputs_used :type Boolean))
  (bind (_inputs_inputs_0 _inputs_inputs_1 _inputs_intputs_2) (break `/Game/Richard/S_InputArrays` (`self.inputs`)))
  (return (and (and (>= tick (`KismetArrayLibrary.Array_Length` _inputs_inputs_0)) (>= tick (`KismetArrayLibrary.Array_Length` _inputs_inputs_1))) (>= tick (`KismetArrayLibrary.Array_Length` _inputs_intputs_2)))))

(fn `get_input`
  (params (tick :type Integer) (character :type Integer))
  (returns (input :type "/Game/Richard/S_InputStruct Structure"))
  (locals (input_array :type "Array of /Game/Richard/S_InputStruct Structure") (input_to_return :type "/Game/Richard/S_InputStruct Structure"))
  (bind (_inputs_inputs_0 _inputs_inputs_1 _inputs_intputs_2) (break `/Game/Richard/S_InputArrays` (`self.inputs`)))
  (bind _tick (`local.tick`))
  (bind _character (`local.character`))
  ; Gets the inputs for the frame from the array for that character
  (if (== character 0)
    (bind _input (`self._get_input_for` _inputs_inputs_0 _tick))
    (set `local.input_to_return` _input)
    (return (`local.input_to_return`))
    (elif (== _character 1)
      (bind _input_2 (`self._get_input_for` _inputs_inputs_1 _tick))
      (set `local.input_to_return` _input_2)
      (return (`local.input_to_return`))
      (elif (== _character 2)
        (bind _input_3 (`self._get_input_for` _inputs_intputs_2 _tick))
        (set `local.input_to_return` _input_3)
        (return (`local.input_to_return`))))))

(fn `reset`
  (bind (_inputs_inputs_0 _inputs_inputs_1 _inputs_intputs_2) (break `/Game/Richard/S_InputArrays` (`self.inputs`)))
  (`KismetArrayLibrary.Array_Clear` _inputs_inputs_0)
  (`KismetArrayLibrary.Array_Clear` _inputs_inputs_1)
  (`KismetArrayLibrary.Array_Clear` _inputs_intputs_2))

(fn `track_input`
  (params (input :type "/Game/Richard/S_InputStruct Structure") (character_id :type Integer))
  (bind (_inputs_inputs_0 _inputs_inputs_1 _inputs_intputs_2) (break `/Game/Richard/S_InputArrays` (`self.inputs`)))
  (if (== character_id 0)
    (`KismetArrayLibrary.Array_Add` _inputs_inputs_0 input)
    (elif (== (`local.character_id`) 1)
      (`KismetArrayLibrary.Array_Add` _inputs_inputs_1 input)
      (elif (== (`local.character_id`) 2)
        (`KismetArrayLibrary.Array_Add` _inputs_intputs_2 input)))))
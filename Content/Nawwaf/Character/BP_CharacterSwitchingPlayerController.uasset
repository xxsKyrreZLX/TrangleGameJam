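; Player controller that lets the player cycle control between all BP_TestCharacter2 characters in the level.
; On BeginPlay it gathers those actors into an array and records the starting player character as the current one.
; Tab calls NextCharacter, which selects the next array index, wraps to the first when out of range, and possesses that character.
; Debug prints show the gathered names and selected indices.
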(event `self.ReceiveBeginPlay`
  (bind _outactors (`GameplayStatics.GetAllActorsOfClass` "/Game/Nawwaf/Character/BP_TestCharacter2.BP_TestCharacter2_C"))
  (set `self.Characters` _outactors)
  (bind _asbp_test_character_2 (cast `/Game/Nawwaf/Character/BP_TestCharacter2` (`GameplayStatics.GetPlayerCharacter` 0)))
  (set `self.CurrentCharacter` _asbp_test_character_2)
  (for _array_element (`self.Characters`)
    (`KismetSystemLibrary.PrintString` (`KismetSystemLibrary.GetDisplayName` _array_element))))

(event `Key|Tab`
  (params (Key :type "Key Structure"))
  (:`Pressed`
    (`self.Next Character`)))

(fn `Next Character`
  (locals (`Local Index` :type Integer))
  (bind _returnvalue (`KismetArrayLibrary.Array_Find` (`self.Characters`) (`self.CurrentCharacter`)))
  (bind _returnvalue_2 (+ _returnvalue 1))
  (set `local.Local Index` 0)
  (bind _output_get (set `local.Local Index` (`KismetMathLibrary.SelectInt` _returnvalue_2 0 (`KismetArrayLibrary.Array_IsValidIndex` (`self.Characters`) _returnvalue_2))))
  (`KismetSystemLibrary.PrintText` (`KismetTextLibrary.Conv_IntToText` _output_get))
  (bind _output (`|GetArrayItem` (`self.Characters`) _output_get))
  (set `self.CurrentCharacter` _output)
  (`self.Possess` _output)
  (`KismetSystemLibrary.PrintText` (`KismetTextLibrary.Conv_IntToText` _returnvalue)))

(fn `UserConstructionScript`)
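; BP_Button is a trigger button actor that changes color when something begins overlapping its Trigger component.
; The overlap calls ChangeColor for green, blue and red, and each call applies its material to slot 0 of the static mesh only if the button itself carries the matching actor tag.
; The overlapping actor is not checked, and nothing in the graph reverts the material.
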(event `self.Trigger.OnComponentBeginOverlap`
  (params (OverlappedComponent :type "PrimitiveComponent Object Reference") (OtherActor :type "Actor Object Reference") (OtherComp :type "PrimitiveComponent Object Reference") (OtherBodyIndex :type Integer) (bFromSweep :type Boolean) (SweepResult :type "HitResult Structure (by ref)"))
  (`self.Change Color` "Green" "/Game/Nawwaf/Materials/MI_ButtonGreen.MI_ButtonGreen")
  (`self.Change Color` "Blue" "/Game/Nawwaf/Materials/MI_ButtonBlue.MI_ButtonBlue")
  (`self.Change Color` "Red" "/Game/Nawwaf/Materials/MI_ButtonRed.MI_ButtonRed"))

(fn `Change Color`
  (params (Color :type Name) (MI :type "MaterialInstance Object Reference"))
  (locals (NewLocalVar :type "MaterialInterface Object Reference" :default "/Script/Engine.MaterialInstanceConstant'/Game/Nawwaf/Materials/MI_ButtonGreen.MI_ButtonGreen'"))
  (if (`self.ActorHasTag` (`local.Color`))
    (`PrimitiveComponent.SetMaterial` (`self.StaticMesh`) 0 (`local.MI`))))

(fn `UserConstructionScript`
  (`parent.UserConstructionScript`))
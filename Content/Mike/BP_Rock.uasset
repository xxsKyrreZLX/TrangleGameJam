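; BP_Rock is a reusable rock that launches on overlap, flies to a target, and can continue on to pop a balloon.
; Timelines lerp it from its start to just above RockTarget, then, on a BalloonCollision overlap, to TargetBalloon, before delayed resets.
; Character-triggered launches store their game time in BP_RockInstance and notify it.
; Boolean flags gate each stage, and disconnected physics and homing attempts remain unused.
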(event `self.ReceiveBeginPlay`
  (set `self.RockLaunch` (`self.K2_GetActorLocation`))
  (set `self.RockEnd` (+ (`self.K2_GetActorLocation` (`self.RockTarget`)) (0.0 0.0 50.0)))
  (`KismetSystemLibrary.PrintString` "Begin Play"))

(event `self.ActorCollision.OnComponentBeginOverlap`
  (params (OverlappedComponent :type "PrimitiveComponent Object Reference") (OtherActor :type "Actor Object Reference") (OtherComp :type "PrimitiveComponent Object Reference") (OtherBodyIndex :type Integer) (bFromSweep :type Boolean) (SweepResult :type "HitResult Structure (by ref)"))
  (if (not (`self.FirstCollision?`))
    (set `self.FirstCollision?` true)
    (if (`self.CanLaunch`)
      ; Stash Time Stamp in Game Instance
      (`self.RockLaunchTime` OtherActor)
      (`PrimitiveComponent.SetSimulatePhysics` (`self.ActorCollision`) false)
      (bind _output_get (set `self.CanLaunch` false))
      (if (not _output_get)
        (bind (_direction _alpha) (`Timeline|RockTravelTimeline` :!via `PlayFromStart`)
          (:`Update`
            (`self.K2_SetActorLocation` (`KismetMathLibrary.VLerp` (`self.RockLaunch`) (`self.RockEnd`) _alpha) false true))
          (:`Finished`
            (set `self.LaunchToBalloon?` true)
            ; ???
            (`KismetSystemLibrary.Delay` (`self.DelayReset`))
            (`self.K2_SetActorLocation` (`self.RockLaunch`) false true)
            (set `self.CanLaunch` true)
            (set `self.LaunchToBalloon?` false)
            (set `self.FirstCollision?` false)
            (`self.SetActorHiddenInGame` false)))))))

(event `self.BalloonCollision.OnComponentBeginOverlap`
  (params (OverlappedComponent :type "PrimitiveComponent Object Reference") (OtherActor :type "Actor Object Reference") (OtherComp :type "PrimitiveComponent Object Reference") (OtherBodyIndex :type Integer) (bFromSweep :type Boolean) (SweepResult :type "HitResult Structure (by ref)"))
  (bind _targetballoon (`self.TargetBalloon`))
  (if (`self.FirstCollision?`)
    (if (`self.LaunchToBalloon?`)
      (set `self.LaunchToBalloon?` false)
      (bind (_direction _alpha) (`Timeline|RockToBalloon` :!via `PlayFromStart`)
        (:`Update`
          (`self.K2_SetActorLocation` (`KismetMathLibrary.VLerp` (`self.RockEnd`) (`self.K2_GetActorLocation` _targetballoon) _alpha))
          (if (< (`self.GetDistanceTo` _targetballoon) (`self.DistanceTolerance`))
            (`/Game/Mike/BP_Balloon.PopBalloon` _targetballoon)
            (`self.SetActorHiddenInGame` true)))
        (:`Finished`
          (`KismetSystemLibrary.Delay` (`self.DelayReset`))
          (`self.K2_SetActorLocation` (`self.RockLaunch`) false true)
          (set `self.CanLaunch` true)
          (set `self.FirstCollision?` false)
          (`self.SetActorHiddenInGame` false))))))

(fn `RockLaunchTime`
  (params (Object :type "Object Object Reference"))
  (returns (CanLaunch :type Boolean))
  (bind _returnvalue (`KismetSystemLibrary.GetGameTimeInSeconds`))
  (cast `Character` Object)
  (bind _asbp_rock_instance (cast `/Game/Mike/BP_RockInstance` (`GameplayStatics.GetGameInstance`)))
  (set `self.RockLaunchTimeLocal` _returnvalue)
  (set `/Game/Mike/BP_RockInstance.RockLaunchTime` _returnvalue _asbp_rock_instance)
  (`/Game/Mike/BP_RockInstance.OnRockLaunchTimeSet` _asbp_rock_instance)
  (return false))

(fn `UserConstructionScript`)
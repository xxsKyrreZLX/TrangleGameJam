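; BP_Balloon is a launchable balloon actor that travels from its start to a target and can be popped by a BP_Rock.
; An ActorCollision overlap starts a timeline lerp, with a delayed return to the origin.
; A RockCollision overlap pops it when balloon and rock are near their endpoints, hiding it, then resetting both.
; Helper functions, gated by Character casts, record launch and pop times in the BP_RockInstance game instance.
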(event `self.ReceiveBeginPlay`
  (set `self.BalloonOrigin` (`self.K2_GetActorLocation`))
  (set `self.BalloonEnd` (`self.K2_GetActorLocation` (`self.BalloonTarget`))))

(event `self.ActorCollision.OnComponentBeginOverlap`
  (params (OverlappedComponent :type "PrimitiveComponent Object Reference") (OtherActor :type "Actor Object Reference") (OtherComp :type "PrimitiveComponent Object Reference") (OtherBodyIndex :type Integer) (bFromSweep :type Boolean) (SweepResult :type "HitResult Structure (by ref)"))
  (if (`self.CanLaunch`)
    ; Stash Time Stamp in Game Instance
    (`self.BalloonLaunchTime` null)
    (bind _output_get (set `self.CanLaunch` false))
    (if (not _output_get)
      (bind (_direction _alpha) (`Timeline|BalloonTravelTimeline` :`NewTime` 1.5 :!via `PlayFromStart`)
        (:`Update`
          (`self.K2_SetActorLocation` (`KismetMathLibrary.VLerp` (`self.BalloonOrigin`) (`self.BalloonEnd`) _alpha))
          (`KismetSystemLibrary.Delay` (`self.ResetDelay`))
          (`self.K2_SetActorLocation` (`self.BalloonOrigin`))
          (set `self.CanLaunch` true))))))

(event `self.RockCollision.OnComponentBeginOverlap`
  (params (OverlappedComponent :type "PrimitiveComponent Object Reference") (OtherActor :type "Actor Object Reference") (OtherComp :type "PrimitiveComponent Object Reference") (OtherBodyIndex :type Integer) (bFromSweep :type Boolean) (SweepResult :type "HitResult Structure (by ref)"))
  (bind _distancetolerance (`self.DistanceTolerance`))
  (`KismetSystemLibrary.PrintString` "BalloonOverlap")
  (if (not (`self.IsPopped`))
    (`self.PopTime` OtherActor)
    (bind _asbp_rock (cast `/Game/Mike/BP_Rock` OtherActor))
    (`KismetSystemLibrary.PrintString` "Cast to BP_Rock")
    (if (and (< (`KismetMathLibrary.VSize` (- (`self.K2_GetActorLocation`) (`self.BalloonEnd`))) _distancetolerance) (< (`KismetMathLibrary.VSize` (- (`self.K2_GetActorLocation` _asbp_rock) (`/Game/Mike/BP_Rock.RockEnd` _asbp_rock))) _distancetolerance))
      (set `self.IsPopped` true)
      (`self.SetActorHiddenInGame` true)
      (`KismetSystemLibrary.Delay` (`self.ResetDelay`))
      (`self.K2_SetActorLocation` (0.0 0.0 0.0) false true)
      (`self.K2_SetActorLocation` _asbp_rock (0.0 0.0 0.0) false false)
      (set `/Game/Mike/BP_Rock.CanLaunch` true _asbp_rock)
      (`self.SetActorHiddenInGame` false)
      (set `self.CanLaunch` true))))

(fn `BalloonLaunchTime`
  (params (Object :type "Object Object Reference"))
  (bind _returnvalue (`KismetSystemLibrary.GetGameTimeInSeconds`))
  (cast `Character` Object)
  (bind _asbp_rock_instance (cast `/Game/Mike/BP_RockInstance` (`GameplayStatics.GetGameInstance`)))
  (set `/Game/Mike/BP_RockInstance.BalloonLaunchTime` _returnvalue _asbp_rock_instance)
  (set `self.BalloonLaunchLocalTime` _returnvalue)
  (`/Game/Mike/BP_RockInstance.OnBalloonLaunchTimeSet` _asbp_rock_instance)
  (return))

(fn `PopTime`
  (params (Object :type "Object Object Reference"))
  (bind _returnvalue (`KismetSystemLibrary.GetGameTimeInSeconds`))
  (cast `Character` Object)
  (`KismetSystemLibrary.PrintString` "Cast to Character")
  (bind _asbp_rock_instance (cast `/Game/Mike/BP_RockInstance` (`GameplayStatics.GetGameInstance`)))
  (`KismetSystemLibrary.PrintString` "Cast to BP_RockInstance")
  (set `self.PopLocalTime` _returnvalue)
  (set `/Game/Mike/BP_RockInstance.PopTime` _returnvalue _asbp_rock_instance)
  (`KismetSystemLibrary.PrintString` "Set Pop Launch Time")
  (`/Game/Mike/BP_RockInstance.OnPopTimeSet` _asbp_rock_instance)
  (return))

(fn `UserConstructionScript`)